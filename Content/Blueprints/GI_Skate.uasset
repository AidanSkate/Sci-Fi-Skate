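; GI_Skate, likely the skate game's Game Instance by its prefix, manages background music that persists across level transitions.
; PlayMusic spawns a persistent 2D sound and stores its audio component, but only when no valid one is already stored.
; SwitchMusic stops any stored track and spawns the new one in its place.
; StopMusic stops the stored component if it is valid.
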(event `Play Music`
  (params (Music :type "SoundBase Object Reference"))
  (`/Engine/EditorBlueprintResources/StandardMacros.IsValid` (`self.Music`)
    (:`Is Not Valid`
      (bind _returnvalue (`GameplayStatics.SpawnSound2D` Music 1.0 1.0 0.0 null true))
      (set `self.Music` _returnvalue))))

(event `SwitchMusic`
  (params (Music :type "SoundBase Object Reference"))
  (bind _music (`self.Music`))
  (`/Engine/EditorBlueprintResources/StandardMacros.IsValid` _music
    (:`Is Valid`
      (`AudioComponent.Stop` _music))
    (:`Is Not Valid`
      _))
  (bind _returnvalue (`GameplayStatics.SpawnSound2D` Music 1.0 1.0 0.0 null true))
  (set `self.Music` _returnvalue))

(event `StopMusic`
  (bind _music (`self.Music`))
  (`/Engine/EditorBlueprintResources/StandardMacros.IsValid` _music
    (:`Is Valid`
      (`AudioComponent.Stop` _music))))