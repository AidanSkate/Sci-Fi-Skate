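; BP_Chest is an interactable chest that opens the player's collectible widget.
; Actor overlap caches the BP_Player_Hotel, shows its prompt and enables CanTalk, while sphere end-overlap reverses both and unpauses.
; CheckforPlayer, which nothing here calls, tests sphere overlap and TalkAttempt, then shows the widget, pauses the game, swaps Enhanced Input contexts to UI navigation and focuses the Back button in UI-only mode.
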(event `self.ReceiveBeginPlay`
  (`KismetSystemLibrary.Delay` 0.6))

(event `self.ReceiveActorBeginOverlap`
  (params (OtherActor :type "Actor Object Reference"))
  (bind _asbp_player_hotel (cast `/Game/Blueprints/Characters/Player/BP_Player_Hotel` OtherActor))
  (bind _output_get (set `self.Player` _asbp_player_hotel))
  (set `/Game/Blueprints/Characters/Player/BP_Player_Hotel.CanTalk` true _output_get)
  (`Widget.SetVisibility` (`/Game/Blueprints/Characters/Player/BP_Player_Hotel.PromptWidget` _output_get) "Visible"))

(event `self.Sphere.OnComponentEndOverlap`
  (params (OverlappedComponent :type "PrimitiveComponent Object Reference") (OtherActor :type "Actor Object Reference") (OtherComp :type "PrimitiveComponent Object Reference") (OtherBodyIndex :type Integer))
  (bind _asbp_player_hotel (cast `/Game/Blueprints/Characters/Player/BP_Player_Hotel` OtherActor))
  (`Widget.SetVisibility` (`/Game/Blueprints/Characters/Player/BP_Player_Hotel.PromptWidget` _asbp_player_hotel) "Collapsed")
  (set `/Game/Blueprints/Characters/Player/BP_Player_Hotel.CanTalk` false _asbp_player_hotel)
  (`GameplayStatics.SetGamePaused` false))

(event `Check for Player`
  (bind _returnvalue (`GameplayStatics.GetPlayerController` 0))
  (bind _player (`self.Player`))
  (bind _returnvalue_2 (pcsubsystem `EnhancedInputLocalPlayerSubsystem` _returnvalue))
  (bind _collectiblewidget (`/Game/Blueprints/Characters/Player/BP_Player_Hotel.CollectibleWidget` _player))
  (if (`PrimitiveComponent.IsOverlappingActor` (`self.Sphere`) (`self.Player`))
    (if (`/Game/Blueprints/Characters/Player/BP_Player_Hotel.TalkAttempt` _player)
      (`Widget.SetVisibility` _collectiblewidget "Visible")
      (`GameplayStatics.SetGamePaused` true)
      (`EnhancedInputSubsystemInterface.RemoveMappingContext` _returnvalue_2 "/Game/Input/IMC_Motel.IMC_Motel" (struct))
      (`EnhancedInputSubsystemInterface.AddMappingContext` _returnvalue_2 "/Game/Input/UINav/IC_UINav.IC_UINav" 0 (struct))
      (`WidgetBlueprintLibrary.SetInputMode_UIOnlyEx` _returnvalue (`/Game/Blueprints/UI/UI_Collectibles.BTN_Back` _collectiblewidget)))))

(fn `UserConstructionScript`)