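; BP_Collectible is a pickup that bobs between two marker points and is collected when BP_Player overlaps it.
; BeginPlay caches the TopPos and BottomPos world locations, then starts the MoveAnim timeline, which lerps CollectibleSprite between them at a configurable play rate.
; A FlipFlop on the timeline's Finished pin alternates reverse and forward playback for endless motion.
; Overlap by the player plays a collect sound and destroys the actor, without updating any score.
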(event `self.ReceiveBeginPlay`
  (set `self.WorldTopPos` (`SceneComponent.K2_GetComponentLocation` (`self.Top Pos`)))
  (set `self.WorldBottomPos` (`SceneComponent.K2_GetComponentLocation` (`self.Bottom Pos`)))
  (`TimelineComponent.SetPlayRate` (`self.MoveAnim`) (`self.MovePlayRate`))
  (`self.MoveForward`))

(event `self.ReceiveTick`
  (params (DeltaSeconds :type "Float (single-precision)")))

(event `MoveForward`
  (bind (_direction _alpha) (`Timeline|MoveAnim` :!via `PlayFromStart` :!label _label)
    (:`Update`
      (`SceneComponent.K2_SetWorldLocation` (`self.CollectibleSprite`) (`KismetMathLibrary.VLerp` (`self.WorldTopPos`) (`self.WorldBottomPos`) _alpha) false false))
    (:`Finished`
      (`/Engine/EditorBlueprintResources/StandardMacros.FlipFlop`
        (:`A`
          (`self.MoveBack`))
        (:`B`
          (`self.MoveForward`))))))

(event `MoveBack`
  (goto _label :!via `ReverseFromEnd`))

(event `self.CollectibleSprite.OnComponentBeginOverlap`
  (params (OverlappedComponent :type "PrimitiveComponent Object Reference") (OtherActor :type "Actor Object Reference") (OtherComp :type "PrimitiveComponent Object Reference") (OtherBodyIndex :type Integer) (bFromSweep :type Boolean) (SweepResult :type "HitResult Structure (by ref)"))
  (cast `/Game/Blueprints/Characters/Player/BP_Player` OtherActor)
  (`GameplayStatics.PlaySoundAtLocation` "/Game/Assets/SFX/Collect_Cue.Collect_Cue" (`self.K2_GetActorLocation`) (struct) 1.0 1.0 0.0 null null null null)
  (`self.K2_DestroyActor`))

(fn `UserConstructionScript`)