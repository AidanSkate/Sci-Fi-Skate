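; BP_MirageStep is a platform cube that toggles between solid and phantom states.
; A Visible flag sets the look and collision: solid blue with physics collision when true, translucent orange with no collision when false.
; BeginPlay caches the player as BP_Player, stopping if the cast fails, then applies the initial state.
; The SwitchCollision event flips the flag and reapplies material and collision.
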(event `self.ReceiveBeginPlay`
  (bind _asbp_player (cast `/Game/Blueprints/Characters/Player/BP_Player` (`GameplayStatics.GetPlayerCharacter` 0)))
  (set `self.Owning Player` _asbp_player)
  (if (`self.Visible?`)
    (`PrimitiveComponent.SetMaterial` (`self.Cube`) 0 "/Game/Assets/Materials/SciFi-Blue.SciFi-Blue")
    (`PrimitiveComponent.SetCollisionEnabled` (`self.Cube`) "QueryAndPhysics")
    (else
      (`PrimitiveComponent.SetMaterial` (`self.Cube`) 0 "/Game/Assets/Materials/SciFi-Orange_Translucent.SciFi-Orange_Translucent")
      (`PrimitiveComponent.SetCollisionEnabled` (`self.Cube`) "NoCollision"))))

(event `SwitchCollision`
  (if (`self.Visible?`)
    (set `self.Visible?` false)
    (else
      (set `self.Visible?` true)))
  (if (`self.Visible?`)
    (`PrimitiveComponent.SetMaterial` (`self.Cube`) 0 "/Game/Assets/Materials/SciFi-Blue.SciFi-Blue")
    (`PrimitiveComponent.SetCollisionEnabled` (`self.Cube`) "QueryAndPhysics")
    (else
      (`PrimitiveComponent.SetMaterial` (`self.Cube`) 0 "/Game/Assets/Materials/SciFi-Orange_Translucent.SciFi-Orange_Translucent")
      (`PrimitiveComponent.SetCollisionEnabled` (`self.Cube`) "NoCollision"))))

(fn `UserConstructionScript`)