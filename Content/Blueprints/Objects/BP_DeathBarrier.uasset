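; BP_DeathBarrier is a kill volume that ends the player's run and restarts the level.
; When BP_Player overlaps its DeathBox, it disables the player's actions, plays a death animation override and plays a 2D death sound.
; It then triggers the FadeOut animation on the main UI held by GM_Skate, waits briefly and reloads via the restartlevel console command.
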(event `self.DeathBox.OnComponentBeginOverlap`
  (params (OverlappedComponent :type "PrimitiveComponent Object Reference") (OtherActor :type "Actor Object Reference") (OtherComp :type "PrimitiveComponent Object Reference") (OtherBodyIndex :type Integer) (bFromSweep :type Boolean) (SweepResult :type "HitResult Structure (by ref)"))
  (bind _asbp_player (cast `/Game/Blueprints/Characters/Player/BP_Player` OtherActor))
  (set `/Game/Blueprints/Characters/Player/BP_Player.CanAct?` false _asbp_player)
  (`PaperZDAnimInstance.K2_PlayAnimationOverride` (`PaperZDCharacter.GetAnimInstance` _asbp_player) "/Game/Blueprints/Characters/Player/AnimSequences/Death.Death" "DefaultSlot" 1.0 0.0)
  (`GameplayStatics.PlaySound2D` "/Game/Assets/SFX/Player/Death_Cue.Death_Cue" 1.0 1.0 0.0 null null)
  (bind _asgm_skate (cast `/Game/Blueprints/GM_Skate` (`GameplayStatics.GetGameMode`)))
  (bind _ui_main (`/Game/Blueprints/GM_Skate.UI_Main` _asgm_skate))
  (`UserWidget.PlayAnimation` _ui_main (`/Game/Blueprints/UI/UI_Main.FadeOut` _ui_main) 0.0 1 "Forward" 1.0 false)
  (`KismetSystemLibrary.Delay` 1.2)
  (`KismetSystemLibrary.ExecuteConsoleCommand` "restartlevel" null))

(fn `UserConstructionScript`)