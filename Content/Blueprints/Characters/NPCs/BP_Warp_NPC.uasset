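; BP_Warp_NPC is an NPC that warps the player to another level in response to a dialogue event.
; On BeginPlay it caches the first UI_FadeOut widget it finds.
; OnDialogueEvent routes the Level Transition event to LevelTransition, passing WarpLevelName.
; That event plays the widget's sped-up FadeOut animation and opens the level by name once it finishes.
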(event `self.ReceiveBeginPlay`
  (`parent.ReceiveBeginPlay`)
  (bind _foundwidgets (`WidgetBlueprintLibrary.GetAllWidgetsOfClass` "/Game/Blueprints/UI/UI_FadeOut.UI_FadeOut_C"))
  (set `self.FadeOutWidget` (`|GetArrayItem` _foundwidgets)))

(event `LevelTransition`
  (params (LevelName :type Name))
  (bind _fadeoutwidget (`self.FadeOutWidget`))
  (`|PlayAnimation` _fadeoutwidget (`/Game/Blueprints/UI/UI_FadeOut.FadeOut` _fadeoutwidget) 0.0 1 "Forward" 1.5
    (:`Finished`
      (`GameplayStatics.OpenLevel` LevelName))))

(fn `OnDialogueEvent`
  (params (Context :type "DlgContext Object Reference") (EventName :type Name))
  (returns (ReturnValue :type Boolean))
  (`|SwitchDialogueCallbackEvent` EventName
    (:`Default`
      (return false))
    (:`LevelTransition`
      (`self.LevelTransition` (`self.WarpLevelName`)))))

(fn `UserConstructionScript`
  (`parent.UserConstructionScript`))