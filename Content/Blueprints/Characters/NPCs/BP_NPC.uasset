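; BP_NPC is a talkable sprite NPC and dialogue participant for BP_Player_Hotel.
; DialogueSphere overlaps set the player's CanTalk and CurrentNPC; Tick starts this NPC's Dialogue when an overlapping player attempts to talk.
; Tick also sets sprite yaw from the Z component of the player's spring-arm forward vector.
; Participant functions return name, display name and gender, value and condition functions are stubs, and WarpLevel opens a named level.
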(event `self.ReceiveBeginPlay`
  (`parent.ReceiveBeginPlay`)
  (bind _returnvalue (`GameplayStatics.GetActorOfClass` "/Game/Blueprints/Characters/Player/BP_Player_Hotel.BP_Player_Hotel_C"))
  (set `self.PlayerChar` _returnvalue))

(event `self.ReceiveTick`
  (params (DeltaSeconds :type "Float (single-precision)"))
  (bind (_returnvalue_roll _returnvalue_pitch) (`KismetMathLibrary.BreakRotator` (`self.K2_GetActorRotation`)))
  (bind _playerchar (`self.PlayerChar`))
  (bind (_returnvalue_x _returnvalue_y _returnvalue_z) (`KismetMathLibrary.BreakVector` (`SceneComponent.GetForwardVector` (`/Game/Blueprints/Characters/Player/BP_Player_Hotel.SpringArm` (`self.PlayerChar`)))))
  (`parent.ReceiveTick` DeltaSeconds)
  (`SceneComponent.K2_SetWorldRotation` (`self.Sprite`) (`KismetMathLibrary.MakeRotator` _returnvalue_roll _returnvalue_pitch _returnvalue_z) false false)
  (if (and (and (`/Game/Blueprints/Characters/Player/BP_Player_Hotel.TalkAttempt` _playerchar) (`/Game/Blueprints/Characters/Player/BP_Player_Hotel.CanTalk` _playerchar)) (`PrimitiveComponent.IsOverlappingActor` (`self.Dialogue Sphere`) _playerchar))
    (`/Game/Blueprints/Characters/Player/BP_Player_Hotel.Start Dialogue with NPC` (`self.PlayerChar`) (`self.Dialogue`) self)))

(event `self.Dialogue Sphere.OnComponentBeginOverlap`
  (params (OverlappedComponent :type "PrimitiveComponent Object Reference") (OtherActor :type "Actor Object Reference") (OtherComp :type "PrimitiveComponent Object Reference") (OtherBodyIndex :type Integer) (bFromSweep :type Boolean) (SweepResult :type "HitResult Structure (by ref)"))
  (bind _asbp_player_hotel (cast `/Game/Blueprints/Characters/Player/BP_Player_Hotel` OtherActor))
  (set `/Game/Blueprints/Characters/Player/BP_Player_Hotel.CurrentNPC` self _asbp_player_hotel)
  (set `/Game/Blueprints/Characters/Player/BP_Player_Hotel.CanTalk` true _asbp_player_hotel)
  (`KismetSystemLibrary.PrintString` (`KismetSystemLibrary.GetDisplayName` self)))

(event `self.Dialogue Sphere.OnComponentEndOverlap`
  (params (OverlappedComponent :type "PrimitiveComponent Object Reference") (OtherActor :type "Actor Object Reference") (OtherComp :type "PrimitiveComponent Object Reference") (OtherBodyIndex :type Integer))
  (bind _asbp_player_hotel (cast `/Game/Blueprints/Characters/Player/BP_Player_Hotel` OtherActor))
  (set `/Game/Blueprints/Characters/Player/BP_Player_Hotel.CanTalk` false _asbp_player_hotel))

(fn `CheckCondition`
  (params (Context :type "DlgContext Object Reference") (ConditionName :type Name))
  (returns (ReturnValue :type Boolean))
  (return false))

(fn `GetBoolValue`
  (params (ValueName :type Name))
  (returns (ReturnValue :type Boolean))
  (return false))

(fn `GetFloatValue`
  (params (ValueName :type Name))
  (returns (ReturnValue :type "Float (single-precision)"))
  (return 0.0))

(fn `GetIntValue`
  (params (ValueName :type Name))
  (returns (ReturnValue :type Integer))
  (return 0))

(fn `GetNameValue`
  (params (ValueName :type Name))
  (returns (ReturnValue :type Name))
  (return "None"))

(fn `GetParticipantDisplayName`
  (params (ActiveSpeaker :type Name))
  (returns (ReturnValue :type Text))
  (return (`self.NPCDisplayName`)))

(fn `GetParticipantGender`
  (returns (ReturnValue :type "ETextGender Enum"))
  (return "Masculine"))

(fn `GetParticipantIcon`
  (params (ActiveSpeaker :type Name) (ActiveSpeakerState :type Name))
  (returns (ReturnValue :type "Texture2D Object Reference"))
  (return null))

(fn `GetParticipantName`
  (returns (ReturnValue :type Name))
  (return (`self.NPCName`)))

(fn `ModifyBoolValue`
  (params (ValueName :type Name) (bNewValue :type Boolean))
  (returns (ReturnValue :type Boolean))
  (return false))

(fn `ModifyFloatValue`
  (params (ValueName :type Name) (bDelta :type Boolean) (Value :type "Float (single-precision)"))
  (returns (ReturnValue :type Boolean))
  (return false))

(fn `ModifyIntValue`
  (params (ValueName :type Name) (bDelta :type Boolean) (Value :type Integer))
  (returns (ReturnValue :type Boolean))
  (return false))

(fn `ModifyNameValue`
  (params (ValueName :type Name) (NameValue :type Name))
  (returns (ReturnValue :type Boolean))
  (return false))

(fn `OnDialogueEvent`
  (params (Context :type "DlgContext Object Reference") (EventName :type Name))
  (returns (ReturnValue :type Boolean))
  (`|SwitchDialogueCallbackEvent` EventName
    (:`Default`
      (return false))))

(fn `UserConstructionScript`
  (`parent.UserConstructionScript`))

(fn `WarpLevel`
  (params (LevelName :type Name))
  (`GameplayStatics.OpenLevel` LevelName))