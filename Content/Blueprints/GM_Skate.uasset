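; GM_Skate is the skate game's game mode, which sets up the save data and main UI when play begins.
; On BeginPlay it loads the BP_SkateSave from slot "1", or creates and saves a new one if none exists, and keeps it in OwningSaveRef.
; Both paths then create the UI_Main widget and add it to the viewport, though a failed cast of the loaded save skips this step.
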(event `self.ReceiveBeginPlay`
  (bind _returnvalue (`GameplayStatics.DoesSaveGameExist` "1"))
  (if _returnvalue
    (bind _returnvalue_2 (`GameplayStatics.LoadGameFromSlot` "1"))
    (bind _asbp_skate_save (cast `/Game/Blueprints/BP_SkateSave` _returnvalue_2))
    (set `self.Owning Save Ref` _asbp_skate_save)
    (else
      (bind _returnvalue_3 (`GameplayStatics.CreateSaveGameObject` "/Game/Blueprints/BP_SkateSave.BP_SkateSave_C"))
      (bind _output_get (set `self.Owning Save Ref` _returnvalue_3))
      (`GameplayStatics.SaveGameToSlot` _output_get "1")))
  (bind _returnvalue_4 (`|CreateWidget` "/Game/Blueprints/UI/UI_Main.UI_Main_C"))
  (bind _output_get_2 (set `self.UI_Main` _returnvalue_4))
  (`UserWidget.AddToViewport` _output_get_2 0))

(fn `UserConstructionScript`)